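; BP_Enemy is a stealth-game enemy that checks for the player and is taken out when the player touches it.
; A looping timer fires a debug-drawn line trace from the Head along fixed world X, not its facing, and only prints the detected player's name.
; Player overlap on the Capsule enables Body physics, then after a short delay notifies Manager of the removal and destroys the actor.
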(event `self.ReceiveBeginPlay`
  (`KismetSystemLibrary.K2_SetTimerDelegate` (delegate `DetectPlayer`) 0.5 true true))

(event `DetectPlayer`
  (bind _returnvalue (`SceneComponent.K2_GetComponentLocation` (`self.Head`)))
  (bind _outhit (`KismetSystemLibrary.LineTraceSingleByProfile` :`Start` (+ _returnvalue (50.0 0.0 0.0)) :`End` (+ _returnvalue (1000.0 0.0 0.0)) :`ProfileName` "Pawn" :`DrawDebugType` "ForDuration"))
  (bind _asbp_third_person_character_custom (cast `/Game/StealthGame/Core/Characters/PlayerCharacter/BP_ThirdPersonCharacterCustom` (`.HitActor` (`GameplayStatics.BreakHitResult` _outhit))))
  (`KismetSystemLibrary.PrintString` (`KismetSystemLibrary.GetDisplayName` _asbp_third_person_character_custom)))

(event `self.Capsule.OnComponentBeginOverlap`
  (params (OverlappedComponent :type "PrimitiveComponent Object Reference") (OtherActor :type "Actor Object Reference") (OtherComp :type "PrimitiveComponent Object Reference") (OtherBodyIndex :type Integer) (bFromSweep :type Boolean) (SweepResult :type "HitResult Structure (by ref)"))
  (cast `/Game/StealthGame/Core/Characters/PlayerCharacter/BP_ThirdPersonCharacterCustom` OtherActor)
  (`PrimitiveComponent.SetSimulatePhysics` (`self.Body`) true)
  (`KismetSystemLibrary.Delay` 2.0)
  (`/Game/StealthGame/Characters/Enemies/BP_EnemySpawnManager.RemoveEnemyAndCheck` (`self.Manager`))
  (`self.K2_DestroyActor`))

(fn `UserConstructionScript`)