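; BP_Enemy is a non-pawn enemy Actor that patrols random navigable points and heads toward the player when spotted.
; Timelines lerp its rotation and location directly, pausing between patrol legs, without an AI controller.
; A looping timer line-traces from Cube to Arrow and, on hitting the player character, retargets movement near that position.
; Capsule overlap is empty; the physics, manager-removal and destroy logic is disconnected.
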(event `self.Capsule.OnComponentBeginOverlap`
  (params (OverlappedComponent :type "PrimitiveComponent Object Reference") (OtherActor :type "Actor Object Reference") (OtherComp :type "PrimitiveComponent Object Reference") (OtherBodyIndex :type Integer) (bFromSweep :type Boolean) (SweepResult :type "HitResult Structure (by ref)")))

(event `self.ReceiveBeginPlay`
  ; A simple approach to getting an Actor (non-pawn) to patrol and chase the player.
  (bind _output_get (set `self.PatrolStartLocation` (`self.K2_GetActorLocation`)))
  (set `self.PatrolTargetLocation` _output_get)
  (bind _returnvalue (`KismetSystemLibrary.K2_SetTimerDelegate` (delegate `DetectPlayer`) 0.5 true true))
  (set `self.DetectPlayerHandle` _returnvalue)
  (`self.PatrolRandom`))

(event `DetectPlayer`
  (bind (_patroltargetlocation_x _patroltargetlocation_y _patroltargetlocation_z) (`KismetMathLibrary.BreakVector` (`self.PatrolTargetLocation`)))
  ; A simple approach to getting an Actor (non-pawn) to patrol and chase the player.
  (bind _outhit (`KismetSystemLibrary.LineTraceSingleByProfile` (+ (`SceneComponent.K2_GetComponentLocation` (`self.Cube`)) (50.0 0.0 0.0)) (`SceneComponent.K2_GetComponentLocation` (`self.Arrow`)) "Pawn"))
  (bind _asbp_third_person_character_custom (cast `/Game/StealthGame/Core/Characters/PlayerCharacter/BP_ThirdPersonCharacterCustom` (`.HitActor` (`GameplayStatics.BreakHitResult` _outhit))))
  (set `self.PatrolStartLocation` (`self.K2_GetActorLocation`))
  (bind (_returnvalue_x _returnvalue_y) (`KismetMathLibrary.BreakVector` (- (`self.K2_GetActorLocation` _asbp_third_person_character_custom) (30.0 30.0 0.0))))
  (set `self.PatrolTargetLocation` (`KismetMathLibrary.MakeVector` _returnvalue_x _returnvalue_y _patroltargetlocation_z))
  (`self.MoveToLocation`))

(event `PatrolRandom`
  (bind (_patrolstartlocation_x _patrolstartlocation_y _patrolstartlocation_z) (`KismetMathLibrary.BreakVector` (`self.PatrolStartLocation`)))
  ; A simple approach to getting an Actor (non-pawn) to patrol and chase the player.
  (bind _randomlocation (`NavigationSystemV1.K2_GetRandomLocationInNavigableRadius` (`self.PatrolStartLocation`) 1000.0 null null))
  (set `self.PatrolTargetLocation` (`KismetMathLibrary.MakeVector` (.x _randomlocation) (.y _randomlocation) _patrolstartlocation_z))
  (`self.RotateToFaceLocation`))

(event `RotateToFaceLocation`
  ; A simple approach to getting an Actor (non-pawn) to patrol and chase the player.
  (set `self.CurrentRotation` (`self.K2_GetActorRotation`))
  (set `self.TargetRotation` (`KismetMathLibrary.MakeRotFromX` (- (`self.PatrolTargetLocation`) (`self.PatrolStartLocation`))))
  (bind (_direction _newtrack_2) (`Timeline|UpdateRotationTimeline` :!via `PlayFromStart`)
    (:`Update`
      (`self.K2_SetActorRotation` (`KismetMathLibrary.RLerp` (`self.CurrentRotation`) (`self.TargetRotation`) _newtrack_2)))
    (:`Finished`
      (`self.MoveToLocation`))))

(event `MoveToLocation`
  (bind (_patrolstartlocation_x _patrolstartlocation_y _patrolstartlocation_z) (`KismetMathLibrary.BreakVector` (`self.PatrolStartLocation`)))
  (bind (_patroltargetlocation_x _patroltargetlocation_y) (`KismetMathLibrary.BreakVector` (`self.PatrolTargetLocation`)))
  ; A simple approach to getting an Actor (non-pawn) to patrol and chase the player.
  (bind (_direction _newtrack_2) (`Timeline|Timeline` :!via `PlayFromStart`)
    (:`Update`
      (`self.K2_SetActorLocation` (`KismetMathLibrary.VLerp` (`KismetMathLibrary.MakeVector` _patrolstartlocation_x _patrolstartlocation_y _patrolstartlocation_z) (`KismetMathLibrary.MakeVector` _patroltargetlocation_x _patroltargetlocation_y _patrolstartlocation_z) _newtrack_2)))
    (:`Finished`
      (set `self.PatrolStartLocation` (`self.PatrolTargetLocation`))
      (`KismetSystemLibrary.Delay` 4.0)
      (`self.PatrolRandom`))))

(fn `UserConstructionScript`)