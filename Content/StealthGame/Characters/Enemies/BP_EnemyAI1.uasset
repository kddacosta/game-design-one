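; Stealth-game enemy that patrols target points, chases a seen player and investigates perceived stimuli, changing walk speed for each behavior.
; Tick picks patrol or chase using CanMove, CanChase and PlayerVisible flags, which gate latent AIMoveTo calls with pauses afterwards.
; PawnSensing flags players by tag and clears sight through a retriggerable delay, while AIPerception sends the enemy to stimulus locations.
; Spline and random patrol variants exist but never run.
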(event `GetNextPatrolPointFromSpline`
  (bind _length (`/Game/StealthGame/Characters/Guards/Guard_V2/BP_PatrolSpline.GetSplineLength` (`self.PatrolSpline`)))
  (set `self.CurrentIndex` (mod (+ (`self.CurrentIndex`) 1) _length)))

(event `PatrolWaypoints`
  (`self.MoveToNextPatrolPoint`))

(event `self.PawnSensing.OnSeePawn`
  (params (Pawn :type "Pawn Object Reference"))
  (`|ExecutionSequence`
    (:`then_0`
      (if (`self.ActorHasTag` Pawn "Player")
        (`KismetSystemLibrary.PrintString` "I SEE YOU")
        (set `self.bPlayerVisible` true)
        (else
          (set `self.bPlayerVisible` false))))
    (:`then_1`
      (`KismetSystemLibrary.PrintString` "Must have been the wind.")
      (`KismetSystemLibrary.RetriggerableDelay` 1.0)
      (set `self.bPlayerVisible` false))))

(event `GetNextPatrolPointIndex`
  (set `self.CurrentIndex` (mod (+ (`self.CurrentIndex`) 1) (`KismetArrayLibrary.Array_Length` (`self.PatrolTargetPoints`)))))

(event `MoveToNextPatrolPoint`
  (`self.UpdateWalkSpeed` 200.0)
  (set `self.bCanMove` false)
  (`|AIMoveTo` self (0.0 0.0 0.0) (`|GetArrayItem` (`self.PatrolTargetPoints`) (`self.CurrentIndex`)) 15.0
    (:`OnSuccess`
      (`KismetSystemLibrary.Delay` 4.0)
      (`self.GetNextPatrolPointIndex`)
      (set `self.bCanMove` true))
    (:`OnFail`
      (`KismetSystemLibrary.Delay` 4.0)
      (set `self.bCanMove` true))))

(event `self.ReceiveTick`
  (params (DeltaSeconds :type "Float (single-precision)"))
  (if (`self.bCanMove`)
    (if (`self.bPlayerVisible`)
      (`self.ChasePlayer`)
      (else
        (`self.PatrolWaypoints`)))
    (elif (and (`self.bCanChase`) (`self.bPlayerVisible`))
      (`MovementComponent.StopMovementImmediately` (`self.CharacterMovement`))
      (`self.ChasePlayer`))))

(event `MoveToNextPatrolAlongSpline`
  (`self.UpdateWalkSpeed` 200.0)
  (bind _point_location (`/Game/StealthGame/Characters/Guards/Guard_V2/BP_PatrolSpline.GetLocationofPointAlongSpline` (`self.PatrolSpline`) (`self.CurrentIndex`)))
  (set `self.bCanMove` false)
  (`|AIMoveTo` self _point_location null 15.0
    (:`OnSuccess`
      (`KismetSystemLibrary.Delay` 4.0)
      (`self.GetNextPatrolPointFromSpline`)
      (set `self.bCanMove` true))
    (:`OnFail`
      (`KismetSystemLibrary.Delay` 4.0)
      (set `self.bCanMove` true))))

(event `ChasePlayer`
  (`self.UpdateWalkSpeed` 400.0)
  (set `self.bCanChase` false)
  (set `self.bCanMove` false)
  (`|AIMoveTo` self (0.0 0.0 0.0) (`GameplayStatics.GetPlayerCharacter` 0) 50.0
    (:`OnSuccess`
      _)
    (:`OnFail`
      _))
  (`KismetSystemLibrary.Delay` 2.0)
  (set `self.bCanMove` true)
  (set `self.bCanChase` true))

(event `PatrolRandom`
  (`self.UpdateWalkSpeed` 200.0)
  (set `self.bCanMove` false)
  (`|AIMoveTo` self (`NavigationSystemV1.K2_GetRandomReachablePointInRadius` (`self.K2_GetActorLocation`) 2000.0 null null) null 50.0
    (:`OnSuccess`
      _)
    (:`OnFail`
      _))
  (`KismetSystemLibrary.Delay` 2.0)
  (set `self.bCanMove` true))

(event `self.AIPerception.OnTargetPerceptionUpdated`
  (params (Actor :type "Actor Object Reference") (Stimulus :type "AIStimulus Structure"))
  (if (`self.bCanChase`)
    (`KismetSystemLibrary.PrintString` "INVESTIGATING" true true (struct :`G` 0.66 :`B` 1.0 :`A` 1.0) 4.0)
    (`MovementComponent.StopMovementImmediately` (`self.CharacterMovement`))
    (`self.UpdateWalkSpeed` 250.0)
    (set `self.bCanMove` false)
    (`|AIMoveTo` self (`.StimulusLocation` (break `AIStimulus` Stimulus)) null
      (:`OnSuccess`
        _)
      (:`OnFail`
        _))
    (`KismetSystemLibrary.Delay` 6.0)
    (set `self.bCanMove` true)))

(fn `UpdateWalkSpeed`
  (params (`New Walk Speed` :type "Float (double-precision)"))
  (set `CharacterMovementComponent.MaxWalkSpeed` `New Walk Speed` (`self.CharacterMovement`)))

(fn `UserConstructionScript`)