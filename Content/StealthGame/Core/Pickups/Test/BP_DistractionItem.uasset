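; BP_DistractionItem is a throwable rock the player picks up and throws to create a noise distraction, with debug prints and spheres.
; Overlap asks the character to pick it up, attaching it to the hand with physics off.
; While held, Tick computes a camera-aimed arc velocity and draws the predicted path.
; Throwing re-enables physics and applies that velocity as an impulse; a DoOnce, reset on pickup, limits noise reporting to one hit.
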(event `self.ReceiveTick`
  (params (DeltaSeconds :type "Float (single-precision)"))
  (bind _returnvalue (`SceneComponent.K2_GetComponentLocation` (`self.Rock`)))
  (if (`self.bPickedUp`)
    (bind (_outlaunchvelocity _returnvalue_2) (`GameplayStatics.SuggestProjectileVelocity_CustomArc` _returnvalue (+ _returnvalue (* (`self.GetActorForwardVector` (`GameplayStatics.GetPlayerCameraManager` 0)) 1500.0))))
    (if _returnvalue_2
      (bind _output_get (set `MovementComponent.Velocity` _outlaunchvelocity (`self.ProjectileMovement`)))
      (`GameplayStatics.Blueprint_PredictProjectilePath_Advanced` (make `PredictProjectilePathParams` :`StartLocation` (`SceneComponent.K2_GetComponentLocation` (`self.Rock`)) :`LaunchVelocity` _output_get :`bTraceWithCollision` true :`MaxSimTime` 5.0 :`TraceChannel` "ECC_Visibility" :`DrawDebugType` "ForOneFrame")))))

(event `self.ReceiveBeginPlay`)

(event `self.Rock.OnComponentBeginOverlap`
  (params (OverlappedComponent :type "PrimitiveComponent Object Reference") (OtherActor :type "Actor Object Reference") (OtherComp :type "PrimitiveComponent Object Reference") (OtherBodyIndex :type Integer) (bFromSweep :type Boolean) (SweepResult :type "HitResult Structure (by ref)"))
  (if (not (`self.bPickedUp`))
    (bind _asbp_third_person_character_custom (cast `/Game/StealthGame/Core/Characters/PlayerCharacter/BP_ThirdPersonCharacterCustom` OtherActor))
    (`/Game/StealthGame/Core/Characters/PlayerCharacter/BP_ThirdPersonCharacterCustom.TryToPickUp` _asbp_third_person_character_custom self)
    (`KismetSystemLibrary.PrintString` "Trying to pick up...")))

(event `/Game/StealthGame/Core/Interactables/BPI_Item.Pickup`
  (params (ParentMesh :type "SkeletalMeshComponent Object Reference"))
  (set `self.bPickedUp` true)
  (`self.ResetBounce`)
  (`SceneComponent.K2_AttachToComponent` (`self.Rock`) ParentMesh "hand_r" "SnapToTarget" "KeepRelative" "KeepRelative" true)
  (`PrimitiveComponent.SetSimulatePhysics` (`self.Rock`) false)
  (`PrimitiveComponent.SetCollisionEnabled` (`self.Rock`) "NoCollision") ; Collide with the ground please
  (set `self.bPickedUp` true))

(event `/Game/StealthGame/Core/Interactables/BPI_Item.Drop`
  (bind _rock (`self.Rock`))
  (set `self.DropLocation` (`SceneComponent.K2_GetComponentLocation` _rock))
  (`SceneComponent.K2_DetachFromComponent` _rock "KeepRelative" "KeepRelative" "KeepRelative" true) ; Don't follow the hand anymore
  (`PrimitiveComponent.SetSimulatePhysics` (`self.Rock`) true) ; use gravity to fall
  (`PrimitiveComponent.SetCollisionEnabled` (`self.Rock`) "QueryAndPhysics") ; Collide with the ground please
  (`SceneComponent.K2_SetWorldLocation` (`self.Rock`) (`self.DropLocation`) false false) ; To prevent the can from going to world origin
  (set `self.bPickedUp` false))

(event `Throw`
  (bind _rock (`self.Rock`))
  (set `self.bPickedUp` false)
  (`|ExecutionSequence`
    (:`then_0`
      (set `self.DropLocation` (`SceneComponent.K2_GetComponentLocation` (`self.Rock`))))
    (:`then_1`
      (`SceneComponent.K2_DetachFromComponent` (`self.Rock`) "KeepWorld" "KeepWorld" "KeepRelative" true)
      (`SceneComponent.K2_SetWorldLocation` (`self.Rock`) (`self.DropLocation`) false false)
      (`PrimitiveComponent.SetCollisionEnabled` (`self.Rock`) "QueryAndPhysics")
      (`PrimitiveComponent.SetSimulatePhysics` (`self.Rock`) true))
    (:`then_2`
      (`PrimitiveComponent.AddVelocityChangeImpulseAtLocation` _rock (`MovementComponent.Velocity` (`self.ProjectileMovement`)) (`SceneComponent.K2_GetComponentLocation` _rock) "None"))))

(event `self.Rock.OnComponentHit`
  (params (HitComponent :type "PrimitiveComponent Object Reference") (OtherActor :type "Actor Object Reference") (OtherComp :type "PrimitiveComponent Object Reference") (NormalImpulse :type "Vector Structure") (Hit :type "HitResult Structure (by ref)"))
  (`/Engine/EditorBlueprintResources/StandardMacros.DoOnce` false :!label _label
    (:`Completed`
      (set `self.PathEndLocation` (`.Location` (`GameplayStatics.BreakHitResult` Hit)))
      (`KismetSystemLibrary.DrawDebugSphere` (0.0 0.0 0.0) 32.0)
      (`KismetSystemLibrary.PrintString` "Projectile Bounce" true true (struct :`R` 1.0 :`G` 0.114689 :`A` 1.0) 5.0)
      (`AISense_Hearing.ReportNoiseEvent` (`self.PathEndLocation`) 30.0 self)
      (`KismetSystemLibrary.PrintString` "Making Sound")
      (`KismetSystemLibrary.DrawDebugSphere` (`self.PathEndLocation`) 50.0 12 (struct :`R` 1.0 :`A` 1.0) 10.0))))

(event `ResetBounce`
  (goto _label :!via `Reset`))

(event `/Game/StealthGame/Core/Interactables/BPI_Item.PrimaryAction`
  (params (ref_thirdPersonCharCustom :type "/Game/StealthGame/Core/Characters/PlayerCharacter/BP_ThirdPersonCharacterCustom Object Reference"))
  (`self.Throw`)
  (set `/Game/StealthGame/Core/Characters/PlayerCharacter/BP_ThirdPersonCharacterCustom.HeldItem` null ref_thirdPersonCharCustom) ; Set the player's held item to nothing
)

(event `self.Rock.OnComponentEndOverlap`
  (params (OverlappedComponent :type "PrimitiveComponent Object Reference") (OtherActor :type "Actor Object Reference") (OtherComp :type "PrimitiveComponent Object Reference") (OtherBodyIndex :type Integer)))

(fn `UserConstructionScript`)