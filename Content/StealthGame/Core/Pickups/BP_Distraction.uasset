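; Throwable distraction pickup for a stealth game that makes noise where it lands.
; Overlap asks the player character to pick it up, attaching the mesh to the hand with physics off.
; While held, Tick previews a camera-aimed arc and caches its velocity in ProjectileMovement, which Throw applies as a physics impulse.
; The first hit after each pickup reports a noise event through a DoOnce that Pickup resets, with debug drawing.
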(event `self.Mesh.OnComponentBeginOverlap`
  (params (OverlappedComponent :type "PrimitiveComponent Object Reference") (OtherActor :type "Actor Object Reference") (OtherComp :type "PrimitiveComponent Object Reference") (OtherBodyIndex :type Integer) (bFromSweep :type Boolean) (SweepResult :type "HitResult Structure (by ref)"))
  (if (not (`self.PickedUp`))
    (bind _asbp_third_person_character_custom (cast `/Game/StealthGame/Core/Characters/PlayerCharacter/BP_ThirdPersonCharacterCustom` OtherActor))
    (`/Game/StealthGame/Core/Characters/PlayerCharacter/BP_ThirdPersonCharacterCustom.TryToPickUp` _asbp_third_person_character_custom self)))

(event `/Game/StealthGame/Core/Interactables/BPI_Item.Pickup`
  (params (ParentMesh :type "SkeletalMeshComponent Object Reference"))
  (`self.ResetBounce`)
  (`SceneComponent.K2_AttachToComponent` (`self.Mesh`) ParentMesh "hand_r" "SnapToTarget" "KeepWorld" "KeepWorld" true)
  (`PrimitiveComponent.SetSimulatePhysics` (`self.Mesh`) false)
  (`PrimitiveComponent.SetCollisionEnabled` (`self.Mesh`) "NoCollision")
  (set `self.PickedUp` true))

(event `/Game/StealthGame/Core/Interactables/BPI_Item.Drop`
  (bind _mesh (`self.Mesh`))
  (set `self.Drop Location` (`SceneComponent.K2_GetComponentLocation` _mesh))
  (`SceneComponent.K2_DetachFromComponent` _mesh "KeepRelative" "KeepRelative" "KeepRelative" true) ; Don't follow the hand anymore
  (`PrimitiveComponent.SetSimulatePhysics` (`self.Mesh`) true) ; use gravity to fall
  (`PrimitiveComponent.SetCollisionEnabled` (`self.Mesh`) "QueryAndPhysics") ; Collide with the ground please
  (`SceneComponent.K2_SetWorldLocation` (`self.Mesh`) (`self.Drop Location`) false false) ; To prevent the can from going to world origin
  (set `self.PickedUp` false))

(event `Throw`
  (bind _mesh (`self.Mesh`))
  (set `self.PickedUp` false)
  (`|ExecutionSequence`
    (:`then_0`
      (set `self.Drop Location` (`SceneComponent.K2_GetComponentLocation` (`self.Mesh`))))
    (:`then_1`
      (`SceneComponent.K2_DetachFromComponent` (`self.Mesh`) "KeepWorld" "KeepWorld" "KeepRelative" true) ; Don't follow the hand anymore
      (`SceneComponent.K2_SetWorldLocation` (`self.Mesh`) (`self.Drop Location`) false false) ; To prevent the can from going to world origin
      (`PrimitiveComponent.SetCollisionEnabled` (`self.Mesh`) "QueryAndPhysics") ; Collide with the ground please
      (`PrimitiveComponent.SetSimulatePhysics` (`self.Mesh`) true) ; use gravity to fall
    )
    (:`then_2`
      (`PrimitiveComponent.AddVelocityChangeImpulseAtLocation` _mesh (`MovementComponent.Velocity` (`self.ProjectileMovement`)) (`SceneComponent.K2_GetComponentLocation` _mesh) "None"))))

(event `self.ReceiveTick`
  (params (DeltaSeconds :type "Float (single-precision)"))
  (bind _returnvalue (`SceneComponent.K2_GetComponentLocation` (`self.Mesh`)))
  (if (`self.PickedUp`)
    (bind (_outlaunchvelocity _returnvalue_2) (`GameplayStatics.SuggestProjectileVelocity_CustomArc` _returnvalue (+ _returnvalue (* (`self.GetActorForwardVector` (`GameplayStatics.GetPlayerCameraManager` 0)) 1500.0))))
    (if _returnvalue_2
      (bind _output_get (set `MovementComponent.Velocity` _outlaunchvelocity (`self.ProjectileMovement`)))
      (`GameplayStatics.Blueprint_PredictProjectilePath_Advanced` (make `PredictProjectilePathParams` :`StartLocation` (`SceneComponent.K2_GetComponentLocation` (`self.Mesh`)) :`LaunchVelocity` _output_get :`bTraceWithCollision` true :`MaxSimTime` 5.0 :`TraceChannel` "ECC_Visibility" :`DrawDebugType` "ForOneFrame")))))

(event `self.ReceiveBeginPlay`)

(event `/Game/StealthGame/Core/Interactables/BPI_Item.PrimaryAction`
  (params (ref_thirdPersonCharCustom :type "/Game/StealthGame/Core/Characters/PlayerCharacter/BP_ThirdPersonCharacterCustom Object Reference"))
  (`self.Throw`)
  (set `/Game/StealthGame/Core/Characters/PlayerCharacter/BP_ThirdPersonCharacterCustom.HeldItem` null ref_thirdPersonCharCustom) ; Set the player's held item to nothing
)

(event `self.ProjectileMovement.OnProjectileStop`
  (params (ImpactResult :type "HitResult Structure (by ref)"))
  (`KismetSystemLibrary.DrawDebugSphere` (`.Location` (`GameplayStatics.BreakHitResult` ImpactResult)) 32.0)
  (`KismetSystemLibrary.PrintString` "PROJECTILE STOP" true true (struct :`R` 1.0 :`B` 0.113469 :`A` 1.0) 5.0))

(event `self.ProjectileMovement.OnProjectileBounce`
  (params (ImpactResult :type "HitResult Structure (by ref)") (ImpactVelocity :type "Vector Structure (by ref)"))
  (`KismetSystemLibrary.DrawDebugSphere` (`.Location` (`GameplayStatics.BreakHitResult` ImpactResult)) 32.0)
  (`KismetSystemLibrary.PrintString` "PROJECTILE BOUNCE" true true (struct :`R` 1.0 :`B` 0.113469 :`A` 1.0) 5.0))

(event `self.ProjectileMovement.OnComponentActivated`
  (params (Component :type "ActorComponent Object Reference") (bReset :type Boolean))
  (`KismetSystemLibrary.PrintString` "PROJECTILE ACTIVATED" true true (struct :`R` 1.0 :`B` 0.113469 :`A` 1.0) 5.0))

(event `self.Mesh.OnComponentHit`
  (params (HitComponent :type "PrimitiveComponent Object Reference") (OtherActor :type "Actor Object Reference") (OtherComp :type "PrimitiveComponent Object Reference") (NormalImpulse :type "Vector Structure") (Hit :type "HitResult Structure (by ref)"))
  (bind _pathendlocation (`self.PathEndLocation`))
  (`/Engine/EditorBlueprintResources/StandardMacros.DoOnce` false :!label _label
    (:`Completed`
      (bind _output_get (set `self.PathEndLocation` (`.Location` (`GameplayStatics.BreakHitResult` Hit))))
      (`KismetSystemLibrary.DrawDebugSphere` _output_get 32.0)
      (`KismetSystemLibrary.PrintString` "PROJECTILE BOUNCE" true true (struct :`R` 1.0 :`B` 0.113469 :`A` 1.0) 5.0)
      (`AISense_Hearing.ReportNoiseEvent` _pathendlocation 30.0 self 2000.0)
      (`KismetSystemLibrary.PrintString` "MAKING SOUND")
      (`KismetSystemLibrary.DrawDebugSphere` _pathendlocation 50.0 12 (struct :`R` 1.0 :`B` 0.02159 :`A` 1.0) 10.0))))

(event `ResetBounce`
  (goto _label :!via `Reset`))

(fn `UserConstructionScript`)