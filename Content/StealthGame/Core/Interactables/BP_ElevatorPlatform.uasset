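; Elevator platform interactable that travels from a start point to an end point when the custom third-person character enters its trigger sphere.
; The overlap plays a Timeline from its start, lerping the Platform's relative location between the Start and End components' locations.
; After reaching the end, it waits for ElevatorWaitTime, then reverses the Timeline to return the platform.
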(event `MoveElevator`
  (bind (_direction _floattrack) (`Timeline|Timeline` :!via `PlayFromStart` :!label _label)
    (:`Update`
      (`SceneComponent.K2_SetRelativeLocation` (`self.Platform`) (`KismetMathLibrary.VLerp` (`SceneComponent.RelativeLocation` (`self.Start`)) (`SceneComponent.RelativeLocation` (`self.End`)) _floattrack) false false))
    (:`Finished`
      (switch `ETimelineDirection` _direction
        (:`Forward`
          (`KismetSystemLibrary.Delay` (`self.ElevatorWaitTime`))
          (`self.ReverseElevator`))))))

(event `self.ReceiveBeginPlay`)

(event `ReverseElevator`
  (goto _label :!via `ReverseFromEnd`))

(event `self.Sphere.OnComponentBeginOverlap`
  (params (OverlappedComponent :type "PrimitiveComponent Object Reference") (OtherActor :type "Actor Object Reference") (OtherComp :type "PrimitiveComponent Object Reference") (OtherBodyIndex :type Integer) (bFromSweep :type Boolean) (SweepResult :type "HitResult Structure (by ref)"))
  (cast `/Game/StealthGame/Core/Characters/PlayerCharacter/BP_ThirdPersonCharacterCustom` OtherActor)
  (`self.MoveElevator`))

(fn `UserConstructionScript`)