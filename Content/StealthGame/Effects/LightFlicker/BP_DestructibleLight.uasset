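; Destructible light actor that flickers at random and can be removed as a sight stimulus for AI perception.
; A looping timer started on BeginPlay randomly decides whether to flicker, then waits a random delay before replaying a timeline that scales the light source's intensity.
; DisableLight only unregisters the stimuli source from the sight sense; this graph does not switch off the light or handle destruction.
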(event `self.ReceiveBeginPlay`
  (`KismetSystemLibrary.K2_SetTimer` null "FlickerLight" 5.0 true))

(event `DisableLight`
  (`AIPerceptionStimuliSourceComponent.UnregisterFromSense` (`self.AIPerceptionStimuliSource`) "/Script/AIModule.AISense_Sight"))

(event `FlickerLight`
  (if (`KismetMathLibrary.RandomBool`)
    (`KismetSystemLibrary.Delay` (`KismetMathLibrary.RandomFloatInRange` 0.2 20.0))
    (bind (_direction _newtrack_0) (`Timeline|FlickerLightTimeline` :!via `PlayFromStart`)
      (:`Update`
        (`LightComponent.SetIntensity` (`self.LightSource`) (* _newtrack_0 1000.0))))))

(fn `UserConstructionScript`)